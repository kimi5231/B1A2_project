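; Desktop game mode that shows OpenCV image frames on screen actors in the level.
; On BeginPlay it creates a BP_OpenCVWidget and sets that one instance on the Screen widget component of every BP_Screen.
; Each Tick it calls the inherited ReadFrame and pushes ImageTexture into the widget's image brush, keeping the image's size.
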(event EventBeginPlay
  (bind _returnvalue (UserInterface|CreateWidget "/Game/OpenCV/BP_OpenCVWidget.BP_OpenCVWidget_C"))
  (bind _output_get (Variables|Default|SetMainScreen _returnvalue))
  (bind _outactors (Actor|GetAllActorsOfClass "/Game/OpenCV/BP_Screen.BP_Screen_C"))
  (for _array_element _outactors
    (bind _asbp_screen (Utilities|Casting|CastToBP_Screen _array_element))
    (UserInterface|SetWidget (Variables|/Game/OpenCV/BP_Screen.BP_Screen_C|GetScreen _asbp_screen) _output_get)))

(event EventTick
  (params (DeltaSeconds :type Float%20%28single-precision%29))
  (Class|DesktopGameModeBase|ReadFrame)
  (Appearance|SetBrushfromTexture (Variables|/Game/OpenCV/BP_OpenCVWidget.BP_OpenCVWidget_C|GetImageWidget (Variables|Default|GetMainScreen)) (Variables|Default|GetimageTexture) false))

(fn ConstructionScript)